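; BP_BrickWall is a destructible Chaos Geometry Collection brick wall that respawns itself, located in a demo folder.
; Each break event picks a small, mid or big impact sound by fragment mass, with random pitch and shared concurrency, adding Niagara dust for all but the lightest breaks.
; The first break starts a lifespan timer, and EndPlay spawns a fresh copy at the actor's transform.
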(event `self.GeometryCollectionComponent.OnChaosBreakEvent`
  (params (BreakEvent :type "ChaosBreakEvent Structure (by ref)"))
  (if (`KismetMathLibrary.InRange_FloatFloat` BreakEvent_Mass 0.0 500.0 true false)
    (`GameplayStatics.PlaySoundAtLocation` "/Game/_DEMO/Walls/BrickWall/Sounds/SW_0_LittleImpact.SW_0_LittleImpact" (0.0 0.0 0.0) (struct) 1.0 (`KismetMathLibrary.RandomFloatInRange` 0.7 1.2) 0.0 null "/Game/_DEMO/Walls/BrickWall/Sounds/NewSoundConcurrency.NewSoundConcurrency" self null)
    (else
      (if (`KismetMathLibrary.InRange_FloatFloat` 0.0 500.0 1000.0)
        (`GameplayStatics.PlaySoundAtLocation` "/Game/_DEMO/Walls/BrickWall/Sounds/SW_1_MidImpact.SW_1_MidImpact" BreakEvent_Location (struct) 1.0 (`KismetMathLibrary.RandomFloatInRange` 0.8 1.1) 0.0 null "/Game/_DEMO/Walls/BrickWall/Sounds/NewSoundConcurrency.NewSoundConcurrency" self null)
        (else
          (`GameplayStatics.PlaySoundAtLocation` "/Game/_DEMO/Walls/BrickWall/Sounds/SW_2_BigImpact.SW_2_BigImpact" BreakEvent_Location (struct) 1.0 (`KismetMathLibrary.RandomFloatInRange` 0.8 1.1) 0.0 null "/Game/_DEMO/Walls/BrickWall/Sounds/NewSoundConcurrency.NewSoundConcurrency" self null)))
      (`NiagaraFunctionLibrary.SpawnSystemAtLocation` "/Game/_DEMO/Walls/BrickWall/NS_BrickDust.NS_BrickDust" BreakEvent_Location)))
  (`/Engine/EditorBlueprintResources/StandardMacros.DoOnce` false
    (:`Completed`
      (`self.SetLifeSpan` 30.0))))

(event `self.ReceiveEndPlay`
  (params (EndPlayReason :type "EEndPlayReason Enum" :default "Destroyed"))
  (`|SpawnActorFromClass` "BP_BrickWall_C" (`self.GetTransform`) "Undefined" "MultiplyWithRoot" null null))

(fn `UserConstructionScript`)